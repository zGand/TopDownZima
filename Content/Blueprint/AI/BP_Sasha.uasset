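; BP_Sasha is an enemy AI character that chases the player and attacks in melee until killed.
; A repeating AIMoveTo drives pursuit, while Tick checks range and state to play the attack montage, pausing CharacterMovement until it completes.
; DamagePlayer applies hit damage but is not called within this Blueprint.
; Incoming damage reduces clamped health; at zero it disables movement and collision, credits BP_Soldier_01 with a kill, then destroys itself after a delay.
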(event EventBeginPlay
  (AI|AIMoveTo self "0, 0, 0" (Game|GetPlayerCharacter 0) 5.0 false :!label _label
    (:OnSuccess
      (Utilities|FlowControl|Delay 0.2 :!label _label_2)
      (goto _label))
    (:OnFail
      (if (CallFunction|IsAlive)
        (goto _label_2)))))

(event EventTick
  (params (DeltaSeconds :type Float%20%28single-precision%29))
  (if (CallFunction|CanAttack)
    (CallFunction|DeactivateAIMovement)
    (Animation|Montage|PlayMontage (Variables|Character|GetMesh) "/Game/Characters/Enemy_Great_Spider/Animations/SashaAttack1.SashaAttack1"
      (:OnCompleted
        (CallFunction|ActivateAIMovement)))))

(event Game|Damage|EventAnyDamage
  (params (Damage :type Float%20%28single-precision%29) (DamageType :type Damage%20Type%20Object%20Reference) (InstigatedBy :type Controller%20Object%20Reference) (DamageCauser :type Actor%20Object%20Reference))
  (bind _output_get (CallFunction|DecreaseHealth Damage))
  (if (== _output_get 0.0)
    (CallFunction|AIDead)
    (Utilities|FlowControl|Delay 2.0)
    (Actor|DestroyActor)))

(fn ConstructionScript)

(fn IsWithinAttackRange
  (return (< (Transformation|GetDistanceTo (Game|GetPlayerCharacter 0)) (Variables|Default|GetAttack%20Range))))

(fn IsAttacking
  (return (Animation|Montage|MontageIsPlaying (Components|SkeletalMesh|GetAnimInstance (Variables|Character|GetMesh)) "/Game/Characters/Enemy_Great_Spider/Animations/SashaAttack1.SashaAttack1")))

(fn DeactivateAIMovement
  (Components|Activation|Deactivate (Variables|Character|GetCharacterMovement)))

(fn ActivateAIMovement
  (Components|Activation|Activate (Variables|Character|GetCharacterMovement) false))

(fn DamagePlayer
  (if (CallFunction|IsAlive)
    (Game|Damage|ApplyDamage (Game|GetPlayerCharacter 0) (Variables|Default|GetDamagePerHit) 0 0)))

(fn DecreaseHealth
  (params (DemageAmount :type Float%20%28single-precision%29))
  (bind _output_get (Variables|Default|SetHealth (Math|Float|Clamp(Float) (- (Variables|Default|GetHealth) DemageAmount) 0.0 1e+02)))
  (return _output_get))

(fn IsAlive
  (return (not (Variables|Default|GetDead))))

(fn CanAttack
  (return (Math|Boolean|ANDBoolean (CallFunction|IsWithinAttackRange) (not (CallFunction|IsAttacking)) (CallFunction|IsAlive))))

(fn AIDead
  (Variables|Default|SetDead true)
  (CallFunction|DeactivateAIMovement)
  (Collision|SetActorEnableCollision false)
  (bind _asbp_soldier_01 (Utilities|Casting|CastToBP_Soldier_01 (Game|GetPlayerCharacter 0)))
  (Default|IncreaseKills _asbp_soldier_01))